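; BP_Cube is a cube actor that shakes the player's camera when it hits world-static geometry hard.
; Its mesh hit event filters by collision object type and a normal impulse threshold.
; A Gate closes as the shake plays and reopens after a short delay, acting as a cooldown against repeated shakes.
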(event `self.StaticMeshComponent.OnComponentHit`
  (params (HitComponent :type "PrimitiveComponent Object Reference") (OtherActor :type "Actor Object Reference") (OtherComp :type "PrimitiveComponent Object Reference") (NormalImpulse :type "Vector Structure") (Hit :type "HitResult Structure (by ref)"))
  (if (`|EnumEquality` (`PrimitiveComponent.GetCollisionObjectType` OtherComp) "ECC_WorldStatic")
    (if (> (`KismetMathLibrary.VSize` NormalImpulse) 20000.0)
      (`/Engine/EditorBlueprintResources/StandardMacros.Gate` false :!label _label
        (:`Exit`
          (`|ExecutionSequence`
            (:`then_0`
              (goto _label :!via `Close`))
            (:`then_1`
              (`PlayerCameraManager.PlayCameraShake` :`self` (`GameplayStatics.GetPlayerCameraManager` 0) :`ShakeClass` "/Game/TomsThrooooow/Blueprints/Gameplay/TestCameraShake.TestCameraShake_C" :`Scale` 1.0)
              (`KismetSystemLibrary.Delay` 1.0)
              (goto _label :!via `Open`))))))))

(fn `UserConstructionScript`)